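; BP_Torch is a torch that makes its point light flicker while the player is within range.
; A self-restarting Flicker event picks a random intensity after a short random delay, then a timeline eases the light toward it with sinusoidal in-out blending.
; Beyond the PlayerDistance threshold, it skips the light update and rechecks every few seconds, limiting work for distant torches.
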(event `self.ReceiveBeginPlay`
  (bind _returnvalue (`GameplayStatics.GetActorOfClass` "/Game/ThirdPersonBP/Blueprints/ThirdPersonCharacter.ThirdPersonCharacter_C"))
  (set `self.player ref` _returnvalue)
  (`self.flicker`))

(event `flicker`
  ;[1 1 1] Flicker (Ruben)
  (if (<= (`self.player distance`) 2000.0)
    (`KismetSystemLibrary.Delay` (`KismetMathLibrary.RandomFloatInRange` 0.0 0.2))
    (set `self.old intencity` (`LightComponentBase.Intensity` (`self.PointLight`)))
    (set `self.new intensity` (`KismetMathLibrary.RandomFloatInRange` 12.5 25.0))
    (`ActorComponent.SetComponentTickInterval` (`self.Flicker timeline`) 0.05)
    (bind (_direction _alpha) (`Timeline|Flicker timeline` :!via `PlayFromStart`)
      (:`Update`
        (`LightComponent.SetIntensity` (`self.PointLight`) (`|EaseFunction` "SinusoidalInOut" _alpha (`self.old intencity`) (`self.new intensity`))))
      (:`Finished`
        (`KismetSystemLibrary.Delay` 0.0)
        (`self.flicker` :!label _label)))
    (else
      (`KismetSystemLibrary.Delay` 3.0)
      (goto _label))))

(fn `UserConstructionScript`)